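; Base enemy character Blueprint with a melee attack and sprint control.
; Attack plays a kick montage on the mesh and calls the OnAttackEnd dispatcher whether it completes or is interrupted.
; StartSprint and StopSprint switch max walk speed between sprint and walk values.
; Health and attack-token functions are stubs: health returns zero, token reservation always fails and token return does nothing.
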(event `Attack`
  (`|PlayMontage` (`self.Mesh`) "/Game/Animations/AnimazioniProva/H2H_Kick01_Montage.H2H_Kick01_Montage"
    (:`OnCompleted`
      _)
    (:`OnInterrupted`
      _))
  (`self.OnAttackEnd`))

(event `/Game/DamageSystem/BPI_Damagiable.ReturnAttackToken`
  (params (Ammount :type Integer)))

(fn `GetCurrentHealth`
  (returns (Health :type "Float (double-precision)"))
  (return 0.0))

(fn `ReserveAttackToken`
  (params (Ammount :type Integer))
  (returns (Success :type Boolean))
  (return false))

(fn `StartSprint`
  (set `CharacterMovementComponent.MaxWalkSpeed` (`self.SprintSpeed`) (`self.CharacterMovement`)))

(fn `StopSprint`
  (set `CharacterMovementComponent.MaxWalkSpeed` (`self.WalkSpeed`) (`self.CharacterMovement`)))

(fn `UserConstructionScript`)