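; Turret actor that turns to face the third-person player while they are within range, with no firing logic.
; It caches the player on BeginPlay, then each Tick checks distance, yaws its root toward them and swaps the head material, restoring brushed metal out of range.
; In range it also runs a debug-drawn sphere trace whose result is ignored, and prints messages, including a taunt based on relative yaw.
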(event `self.ReceiveBeginPlay`
  (bind _asbp_third_person_character (cast `/Game/ThirdPerson/Blueprints/BP_ThirdPersonCharacter` (`GameplayStatics.GetPlayerCharacter` 0)))
  (set `self.As BP Third Person Character` _asbp_third_person_character))

(event `self.ReceiveTick`
  (params (DeltaSeconds :type "Float (single-precision)"))
  (bind (_returnvalue_roll _returnvalue_pitch _returnvalue_yaw) (`KismetMathLibrary.BreakRotator` (`SceneComponent.K2_GetComponentRotation` (`self.Cylinder3`))))
  (bind (_returnvalue_roll_2 _returnvalue_pitch_2 _returnvalue_yaw_2) (`KismetMathLibrary.BreakRotator` (`SceneComponent.K2_GetComponentRotation` (`Character.CapsuleComponent` (`self.As BP Third Person Character`)))))
  (bind _returnvalue (- _returnvalue_yaw_2 _returnvalue_yaw))
  (if (<= (`KismetMathLibrary.VSize` (- (`SceneComponent.K2_GetComponentLocation` (`Character.CapsuleComponent` (`self.As BP Third Person Character`))) (`SceneComponent.K2_GetComponentLocation` (`self.DefaultSceneRoot`)))) 1000.0)
    (`SceneComponent.K2_SetRelativeRotation` (`self.DefaultSceneRoot`) (`KismetMathLibrary.MakeRotator` 0.0 0.0 (.yaw (`KismetMathLibrary.MakeRotationFromAxes` (`KismetMathLibrary.Normal` (- (`SceneComponent.K2_GetComponentLocation` (`Actor.RootComponent` (`self.As BP Third Person Character`))) (`SceneComponent.K2_GetComponentLocation` (`self.DefaultSceneRoot`))))))) false false)
    (`PrimitiveComponent.SetMaterial` (`self.Head`) 0 "/DatasmithContent/Materials/AliasReference.AliasReference")
    (`KismetSystemLibrary.SphereTraceSingleForObjects` :`Start` (`SceneComponent.K2_GetComponentLocation` (`self.Cylinder3`)) :`End` (`SceneComponent.K2_GetComponentLocation` (`Character.CapsuleComponent` (`self.As BP Third Person Character`))) :`Radius` 20.0 :`ObjectTypes` (`|MakeArray` "ObjectTypeQuery3" :!type "EObjectTypeQuery Enum") :`DrawDebugType` "ForDuration")
    (`KismetSystemLibrary.PrintString` "preso")
    (if (and (<= _returnvalue -80.0) (>= _returnvalue -100.0))
      (`KismetSystemLibrary.PrintString` "Minchia Guardi?"))
    (else
      (`PrimitiveComponent.SetMaterial` (`self.Head`) 0 "/DatasmithContent/Materials/FBXImporter/VRED/BrushedMetal.BrushedMetal"))))

(fn `UserConstructionScript`)